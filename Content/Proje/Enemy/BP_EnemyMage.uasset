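; Mage enemy actor that starts a battle when the player character enters its sphere and takes elemental damage during it.
; The overlap sets the combat-state struct, adds the interface and button widgets, reveals the health bar and notifies the player.
; Three button events subtract fire, ice or air damage from the health struct, while Tick refreshes the bar.
; At zero health it removes both screen widgets, signals battle end and destroys itself.
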(event `self.ReceiveBeginPlay`
  (bind (`_s_savaştamıyız_maxhp` `_s_savaştamıyız_hp` `_s_savaştamıyız_maxmana` `_s_savaştamıyız_mana` `_s_savaştamıyız_strength` `_s_savaştamıyız_savaştamıyız`) (break `/Game/Proje/Structer/S_Stats` (`self.S_Savaştamıyız`)))
  (`SceneComponent.SetVisibility` (`self.Widget`) `_s_savaştamıyız_savaştamıyız` false))

(event `self.ReceiveTick`
  (params (DeltaSeconds :type "Float (single-precision)"))
  (bind (_s_health_name _s_health_health _s_health_maxhealth) (break `/Game/Proje/Structer/S_EnemyMage` (`self.S_Health`)))
  ; Progres Bar
  (bind _aswb_enemy_hud (cast `/Game/Proje/Widgets/WB_EnemyHud` (`WidgetComponent.GetWidget` (`self.Widget`))))
  (`ProgressBar.SetPercent` (`/Game/Proje/Widgets/WB_EnemyHud.HealthBar` _aswb_enemy_hud) (/ _s_health_health _s_health_maxhealth)))

(event `Öldün`
  (`Widget.RemoveFromParent` (`self.ButtonRef`))
  (`Widget.RemoveFromParent` (`self.ArayüzRef`))
  (bind _outactors (`GameplayStatics.GetAllActorsOfClass` "/Game/ThirdPerson/Blueprints/BP_ThirdPersonCharacter.BP_ThirdPersonCharacter_C"))
  (`/Game/ThirdPerson/Blueprints/BP_ThirdPersonCharacter.Savaş Bitti` (`|GetArrayItem` _outactors))
  (`self.K2_DestroyActor`))

(event `self.BTN_1`
  (bind (_s_health_name _s_health_health) (break `/Game/Proje/Structer/S_EnemyMage` (`self.S_Health`)))
  (bind _s_hasar_firedamage (break `/Game/Proje/Structer/S_Damage` (`self.S_HASAR`)))
  (bind (_s_health_name_2 _s_health_health_2) (break `/Game/Proje/Structer/S_EnemyMage` (`self.S_Health`)))
  ;[0.02572 0.1014 0.15 0.5] widget arayüz
  (`KismetSystemLibrary.PrintString` "ohayoo11111")
  (set `self.S_Health` (make `/Game/Proje/Structer/S_EnemyMage` "Magel" (- _s_health_health_2 _s_hasar_firedamage)))
  (if (<= _s_health_health 0.0) :!label _label
    (`self.Öldün`)))

(event `self.BTN_2`
  (bind (_s_hasar_firedamage _s_hasar_icedamage) (break `/Game/Proje/Structer/S_Damage` (`self.S_HASAR`)))
  (bind (_s_health_name _s_health_health) (break `/Game/Proje/Structer/S_EnemyMage` (`self.S_Health`)))
  ;[0.02572 0.1014 0.15 0.5] widget arayüz
  (`KismetSystemLibrary.PrintString` "çançinçon22222")
  (set `self.S_Health` (make `/Game/Proje/Structer/S_EnemyMage` "Magel" (- _s_health_health _s_hasar_icedamage)))
  (goto _label))

(event `self.BTN_3`
  (bind (_s_hasar_firedamage _s_hasar_icedamage _s_hasar_airdamage) (break `/Game/Proje/Structer/S_Damage` (`self.S_HASAR`)))
  (bind (_s_health_name _s_health_health) (break `/Game/Proje/Structer/S_EnemyMage` (`self.S_Health`)))
  ;[0.02572 0.1014 0.15 0.5] widget arayüz
  (`KismetSystemLibrary.PrintString` "baraba33333")
  (set `self.S_Health` (make `/Game/Proje/Structer/S_EnemyMage` "Magel" (- _s_health_health _s_hasar_airdamage)))
  (goto _label))

(event `self.Sphere.OnComponentBeginOverlap`
  (params (OverlappedComponent :type "PrimitiveComponent Object Reference") (OtherActor :type "Actor Object Reference") (OtherComp :type "PrimitiveComponent Object Reference") (OtherBodyIndex :type Integer) (bFromSweep :type Boolean) (SweepResult :type "HitResult Structure (by ref)"))
  (bind (`_s_savaştamıyız_maxhp` `_s_savaştamıyız_hp` `_s_savaştamıyız_maxmana` `_s_savaştamıyız_mana` `_s_savaştamıyız_strength` `_s_savaştamıyız_savaştamıyız`) (break `/Game/Proje/Structer/S_Stats` (`self.S_Savaştamıyız`)))
  (cast `/Game/ThirdPerson/Blueprints/BP_ThirdPersonCharacter` OtherActor)
  (set `self.S_Savaştamıyız` (make `/Game/Proje/Structer/S_Stats` 100.0 100.0 3 3 10.0 true))
  (`KismetSystemLibrary.PrintString` "içerde")
  (bind _returnvalue (`|CreateWidget` "/Game/Proje/Widgets/WB_Arayüz.WB_Arayüz_C"))
  (bind _output_get (set `self.ArayüzRef` _returnvalue))
  (`UserWidget.AddToViewport` _output_get 0)
  (bind _returnvalue_2 (`|CreateWidget` "/Game/Proje/Widgets/WB_Button.WB_Button_C"))
  (bind _output_get_2 (set `self.ButtonRef` _returnvalue_2))
  (`UserWidget.AddToViewport` _output_get_2 0)
  (`SceneComponent.SetVisibility` (`self.Widget`) `_s_savaştamıyız_savaştamıyız` false)
  (bind _outactors (`GameplayStatics.GetAllActorsOfClass` "/Game/ThirdPerson/Blueprints/BP_ThirdPersonCharacter.BP_ThirdPersonCharacter_C"))
  (`/Game/ThirdPerson/Blueprints/BP_ThirdPersonCharacter.Savaş Başladı` (`|GetArrayItem` _outactors)))

(fn `UserConstructionScript`)