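; Enemy actor for a spell-based battle, started when the player overlaps its sphere, which opens combat widgets and notifies the character.
; BTN1–3 events apply fire, ice or air damage plus Strength with Niagara effects; fire also enables burn damage on each Yan call.
; Tick refreshes the health bar and text.
; At zero health, Öldün removes the UI, ends the battle, levels up the player and destroys the enemy.
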(event `self.ReceiveBeginPlay`
  (bind (`_s_savaştamıyız_maxhp` `_s_savaştamıyız_hp` `_s_savaştamıyız_maxmana` `_s_savaştamıyız_mana` `_s_savaştamıyız_strength` `_s_savaştamıyız_savaştamıyız`) (break `/Game/Proje/Structer/S_Stats` (`self.S_Savaştamıyız`)))
  (`SceneComponent.SetVisibility` (`self.Widget`) `_s_savaştamıyız_savaştamıyız` false))

(event `self.ReceiveTick`
  (params (DeltaSeconds :type "Float (single-precision)"))
  (bind (_s_health_name _s_health_health _s_health_maxhealth) (break `/Game/Proje/Structer/S_Enemy` (`self.S_Health`)))
  ; Progres Bar
  (bind _aswb_enemy_hud (cast `/Game/Proje/Widgets/WB_EnemyHud` (`WidgetComponent.GetWidget` (`self.Widget`))))
  (`ProgressBar.SetPercent` (`/Game/Proje/Widgets/WB_EnemyHud.HealthBar` _aswb_enemy_hud) (/ _s_health_health _s_health_maxhealth))
  (`TextRenderComponent.K2_SetText` (`self.TextRender`) (`KismetTextLibrary.Conv_DoubleToText` _s_health_health "HalfToEven"))
  (`KismetSystemLibrary.Delay` 1.0)
  (set `self.S_Savaştamıyız` (`self.S_Savaştamıyız`)))

(event `Öldün`
  (`Widget.RemoveFromParent` (`self.ButtonRef`))
  (`Widget.RemoveFromParent` (`self.ArayüzRef`))
  (set `self.Yak` false)
  (if (`self.yanarak öldü`)
    (`ActorComponent.Deactivate` (`self.efecktref`)))
  (bind _outactors (`GameplayStatics.GetAllActorsOfClass` "/Game/ThirdPerson/Blueprints/BP_ThirdPersonCharacter.BP_ThirdPersonCharacter_C"))
  (`/Game/ThirdPerson/Blueprints/BP_ThirdPersonCharacter.Savaş Bitti` (`|GetArrayItem` _outactors))
  (`/Game/ThirdPerson/Blueprints/BP_ThirdPersonCharacter.LvUp` (`self.As BP Third Person Character`))
  (`self.K2_DestroyActor`))

(event `/Game/Proje/Interface/Damage.BTN_1`
  (bind (_s_health_name _s_health_health) (break `/Game/Proje/Structer/S_Enemy` (`self.S_Health`)))
  (bind (`_s_savaştamıyız_maxhp` `_s_savaştamıyız_hp` `_s_savaştamıyız_maxmana` `_s_savaştamıyız_mana` `_s_savaştamıyız_strength`) (break `/Game/Proje/Structer/S_Stats` (`self.S_Savaştamıyız`)))
  (bind (_s_health_name_2 _s_health_health_2) (break `/Game/Proje/Structer/S_Enemy` (`self.S_Health`)))
  (bind _s_hasar_firedamage (break `/Game/Proje/Structer/S_Damage` (`self.S_HASAR`)))
  (bind (_returnvalue_x _returnvalue_y _returnvalue_z) (`KismetMathLibrary.BreakVector` (`SceneComponent.K2_GetComponentLocation` (`self.Mesh`))))
  ;[0.02572 0.1014 0.15 0.5] widget arayüz
  (set `self.S_Health` (make `/Game/Proje/Structer/S_Enemy` "Selim Kurugöt" (- _s_health_health (+ _s_hasar_firedamage `_s_savaştamıyız_strength`))))
  (set `self.Yak` true)
  (`NiagaraFunctionLibrary.SpawnSystemAtLocation` "/Game/Free_Spells/VFX_Niagara/NS_Free_Spells_Explosion.NS_Free_Spells_Explosion" (`KismetMathLibrary.MakeVector` _returnvalue_x _returnvalue_y (+ _returnvalue_z 110.0)) (struct) (0.5 0.5 0.5))
  (if (<= _s_health_health_2 0.0) :!label _label
    (`self.Öldün`)))

(event `/Game/Proje/Interface/Damage.BTN_2`
  (bind (`_s_savaştamıyız_maxhp` `_s_savaştamıyız_hp` `_s_savaştamıyız_maxmana` `_s_savaştamıyız_mana` `_s_savaştamıyız_strength`) (break `/Game/Proje/Structer/S_Stats` (`self.S_Savaştamıyız`)))
  (bind (_s_hasar_firedamage _s_hasar_icedamage) (break `/Game/Proje/Structer/S_Damage` (`self.S_HASAR`)))
  (bind (_s_health_name _s_health_health) (break `/Game/Proje/Structer/S_Enemy` (`self.S_Health`)))
  (bind (_returnvalue_x _returnvalue_y _returnvalue_z) (`KismetMathLibrary.BreakVector` (`SceneComponent.K2_GetComponentLocation` (`self.Mesh`))))
  ;[0.02572 0.1014 0.15 0.5] widget arayüz
  (set `self.S_Health` (make `/Game/Proje/Structer/S_Enemy` "Selim Kurugöt" (- _s_health_health (+ _s_hasar_icedamage `_s_savaştamıyız_strength`))))
  (message `/Game/Proje/Interface/Düşman.Heal` (`self.As BP Third Person Character`))
  (`NiagaraFunctionLibrary.SpawnSystemAtLocation` "/Game/Free_Spells/VFX_Niagara/NS_Free_Spells_Buff_Lightning.NS_Free_Spells_Buff_Lightning" (`KismetMathLibrary.MakeVector` _returnvalue_x _returnvalue_y (+ _returnvalue_z 25.0)) (struct) (5.0 5.0 5.0) false)
  (`NiagaraFunctionLibrary.SpawnSystemAtLocation` "/Game/Free_Spells/VFX_Niagara/NS_Free_Spells_Buff_Healing.NS_Free_Spells_Buff_Healing" (`SceneComponent.K2_GetComponentLocation` (`Character.Mesh` (`GameplayStatics.GetPlayerCharacter` 0))) (struct) (1.0 1.0 1.0) false)
  (goto _label))

(event `/Game/Proje/Interface/Damage.BTN_3`
  (bind (_s_health_name _s_health_health) (break `/Game/Proje/Structer/S_Enemy` (`self.S_Health`)))
  (bind (_s_hasar_firedamage _s_hasar_icedamage _s_hasar_airdamage) (break `/Game/Proje/Structer/S_Damage` (`self.S_HASAR`)))
  (bind (`_s_savaştamıyız_maxhp` `_s_savaştamıyız_hp` `_s_savaştamıyız_maxmana` `_s_savaştamıyız_mana` `_s_savaştamıyız_strength`) (break `/Game/Proje/Structer/S_Stats` (`self.S_Savaştamıyız`)))
  (bind (_returnvalue_x _returnvalue_y _returnvalue_z) (`KismetMathLibrary.BreakVector` (`SceneComponent.K2_GetComponentLocation` (`self.Mesh`))))
  ;[0.02572 0.1014 0.15 0.5] widget arayüz
  (set `self.S_Health` (make `/Game/Proje/Structer/S_Enemy` "Selim Kurugöt" (- _s_health_health (+ _s_hasar_airdamage `_s_savaştamıyız_strength`))))
  (`NiagaraFunctionLibrary.SpawnSystemAtLocation` "/Game/Free_Spells/VFX_Niagara/NS_Free_Spells_Buff_Air.NS_Free_Spells_Buff_Air" (`KismetMathLibrary.MakeVector` _returnvalue_x _returnvalue_y (+ _returnvalue_z 55.0)) (struct) (1.0 1.0 2.0) false)
  (goto _label))

(event `self.Sphere.OnComponentBeginOverlap`
  (params (OverlappedComponent :type "PrimitiveComponent Object Reference") (OtherActor :type "Actor Object Reference") (OtherComp :type "PrimitiveComponent Object Reference") (OtherBodyIndex :type Integer) (bFromSweep :type Boolean) (SweepResult :type "HitResult Structure (by ref)"))
  (bind _asbp_third_person_character (cast `/Game/ThirdPerson/Blueprints/BP_ThirdPersonCharacter` OtherActor))
  (set `self.As BP Third Person Character` _asbp_third_person_character)
  (set `self.S_Savaştamıyız` (`self.S_Savaştamıyız`))
  (`SceneComponent.SetVisibility` (`self.TextRender`) true false)
  (bind _returnvalue (`|CreateWidget` "/Game/Proje/Widgets/WB_Arayüz.WB_Arayüz_C" null null))
  (bind _output_get (set `self.ArayüzRef` _returnvalue))
  (`UserWidget.AddToViewport` _output_get 0)
  (bind _returnvalue_2 (`|CreateWidget` "/Game/Proje/Widgets/WB_Button.WB_Button_C"))
  (bind _output_get_2 (set `self.ButtonRef` _returnvalue_2))
  (`UserWidget.AddToViewport` _output_get_2 0)
  (`SceneComponent.SetVisibility` (`self.Widget`) true false)
  (bind _outactors (`GameplayStatics.GetAllActorsOfClass` "/Game/ThirdPerson/Blueprints/BP_ThirdPersonCharacter.BP_ThirdPersonCharacter_C"))
  (`/Game/ThirdPerson/Blueprints/BP_ThirdPersonCharacter.Savaş Başladı` (`|GetArrayItem` _outactors)))

(event `/Game/Proje/Interface/Düşman.Düşman anim`
  ;[0.6573 0.6082 0.02107 0.5] ANİM
  (`SkeletalMeshComponent.PlayAnimation` (`self.Mesh`) "/Game/SKnight_modular/Skeleton_Knight_05/demo/animations/ThirdPersonWalk.ThirdPersonWalk" false)
  (`KismetSystemLibrary.Delay` 1.0)
  (`SkeletalMeshComponent.PlayAnimation` (`self.Mesh`) "/Game/SKnight_modular/Skeleton_Knight_05/demo/animations/ThirdPersonIdle.ThirdPersonIdle" true))

(event `/Game/Proje/Interface/I_lvUP.HasarArttır`
  (set `self.S_Savaştamıyız` (make `/Game/Proje/Structer/S_Stats` 100.0 100.0 3 3 (+ (`.Strength_13_B559586D49212D4BAE21E58CDD4E027D` (break `/Game/Proje/Structer/S_Stats` (`self.S_Savaştamıyız`))) 50.0))))

(event `/Game/Proje/Interface/Düşman.Yan`
  (bind (_s_health_name _s_health_health) (break `/Game/Proje/Structer/S_Enemy` (`self.S_Health`)))
  (bind (_s_health_name_2 _s_health_health_2 _s_health_maxhealth) (break `/Game/Proje/Structer/S_Enemy` (`self.S_Health`)))
  (bind (_returnvalue_x _returnvalue_y _returnvalue_z) (`KismetMathLibrary.BreakVector` (`SceneComponent.K2_GetComponentLocation` (`self.Mesh`))))
  (if (`self.Yak`)
    (set `self.S_Health` (make `/Game/Proje/Structer/S_Enemy` "Selim Kurugöt" (- _s_health_health_2 50.0) _s_health_maxhealth))
    (if (`self.alevlendi`)
      (`KismetSystemLibrary.PrintString` "YANIYOR")
      (if (<= _s_health_health 0.0)
        (`self.Öldün`)
        (`ActorComponent.Deactivate` (`self.efecktref`)))
      (else
        (bind _returnvalue (`NiagaraFunctionLibrary.SpawnSystemAtLocation` "/Game/Fab/TorchFire/FX/NS_TorchFire_Standard.NS_TorchFire_Standard" (`KismetMathLibrary.MakeVector` (+ _returnvalue_x 10.0) _returnvalue_y (+ _returnvalue_z 110.0)) (struct) (20.0 20.0 10.0) false))
        (set `self.efecktref` _returnvalue)
        (set `self.alevlendi` true)
        (set `self.yanarak öldü` true)))))

(fn `UserConstructionScript`)