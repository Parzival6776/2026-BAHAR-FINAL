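; BP_TurnManager builds a character turn order based on Speed.
; CalculateTurnOrder repeatedly scans UnsortedList for a Speed above HigthSpeed and appends FastestCharacter to SortedList until UnsortedList is empty.
; Each pass removes the UnsortedList entry at the index returned by the SortedList add, rather than the chosen character's index.
; HigthSpeed is not reset between passes.
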(fn `CalculateTurnOrder`
  (while (> (`KismetArrayLibrary.Array_Length` (`self.UnsortedList`)) 0)
    (for _array_element (`self.UnsortedList`)
      (bind _speed (`/Game/Proje/BP_BaseCharacter.Speed` _array_element))
      (if (> _speed (`self.HigthSpeed`))
        (set `self.HigthSpeed` _speed)
        (set `self.FastestCharacter` _array_element)))
    (bind _returnvalue (`KismetArrayLibrary.Array_Add` (`self.SortedList`) (`self.FastestCharacter`)))
    (`KismetArrayLibrary.Array_Remove` (`self.UnsortedList`) _returnvalue)))

(fn `UserConstructionScript`)